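; FuseActor is a Blueprint actor that animates a burning fuse when its Start event is called.
; A timeline drives the "Animate" scalar parameter on the static mesh materials and moves a particle system along the root's forward axis in step with it.
; The particle position runs slightly ahead of the material value, clamped to a small overshoot, and the particles deactivate when the timeline finishes.
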(event `self.ReceiveBeginPlay`)

(event `Start`
  (bind _defaultsceneroot (`self.DefaultSceneRoot`))
  (bind _returnvalue (`SceneComponent.GetForwardVector` _defaultsceneroot))
  (bind (_direction _fusetime) (`Timeline|FuseTimeline` :!via `PlayFromStart`)
    (:`Update`
      (`MeshComponent.SetScalarParameterValueOnMaterials` (`self.StaticMesh`) "Animate" _fusetime)
      (`SceneComponent.K2_SetWorldLocation` (`self.ParticleSystem`) (+ (+ (`SceneComponent.K2_GetComponentLocation` _defaultsceneroot) (* _returnvalue -84.0)) (* (* _returnvalue 2406.0) (`KismetMathLibrary.FClamp` (+ _fusetime 0.1) 0.0 1.05))) false false))
    (:`Finished`
      (`ActorComponent.Deactivate` (`self.ParticleSystem`)))))

(fn `UserConstructionScript`)