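; Runs a timed local-multiplayer round of Beaverlicious, with bomb managers and fuses.
; After a short delay, it creates a player and possessed, recolored third-person character per PlayerStart, then switches to the tagged main camera.
; Fuse timelines are rate-scaled to burn over exactly RoundDuration.
; At round end, it records and prints each player's bomb-slot state and calls EndGame on all managers from inside that loop, so repeatedly.
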(event `self.ReceiveBeginPlay`
  (bind _returnvalue (`GameplayStatics.GetPlayerController` 0))
  (`KismetSystemLibrary.Delay` 1.0)
  (`|ExecutionSequence`
    (:`then_0`
      (`self.SpawnPlayers`)
      (bind _outactors (`GameplayStatics.GetAllActorsOfClass` "/Game/Blueprints/BombManager/BombManager.BombManager_C"))
      (set `self.BombManagers` _outactors)
      (bind _outactors_2 (`GameplayStatics.GetAllActorsOfClassWithTag` "/Script/Engine.CameraActor" "MainCamera"))
      (`PlayerController.SetViewTargetWithBlend` _returnvalue (`|GetArrayItem` _outactors_2) 0.0 "VTBlend_Linear" 0.0 false)
      (set `PlayerController.bShowMouseCursor` false _returnvalue)
      (`WidgetBlueprintLibrary.SetInputMode_GameOnly` _returnvalue))
    (:`then_1`
      (bind _outactors_3 (`GameplayStatics.GetAllActorsOfClass` "/Game/Blueprints/FuseActor/FuseActor.FuseActor_C"))
      (for _array_element _outactors_3
        (bind _fusetimeline (`/Game/Blueprints/FuseActor/FuseActor.FuseTimeline` _array_element))
        (`TimelineComponent.SetPlayRate` _fusetimeline (/ (`TimelineComponent.GetTimelineLength` _fusetimeline) (`self.RoundDuration`)))
        (`/Game/Blueprints/FuseActor/FuseActor.Start` _array_element)))
    (:`then_2`
      (`KismetSystemLibrary.Delay` (`self.RoundDuration`))
      (`KismetSystemLibrary.PrintString` "End Game")
      (for (_array_element_2 _array_index) (`self.BombManagers`)
        (`KismetArrayLibrary.Array_Set` (`self.PlayerBombStates`) _array_index (not (`/Game/Blueprints/BombManager/BombManager.AnySlotFalseOrEmpty` _array_element_2)) true)
        (for _array_element_3 (`self.BombManagers`)
          (`/Game/Blueprints/BombManager/BombManager.EndGame` _array_element_3)))
      (for (_array_element_4 _array_index_2) (`self.PlayerBombStates`)
        (`KismetSystemLibrary.PrintString` (`KismetStringLibrary.Concat_StrStr` (`KismetStringLibrary.Concat_StrStr` (`KismetStringLibrary.Concat_StrStr` "Player " (`KismetStringLibrary.Conv_IntToString` _array_index_2)) "    ") (`KismetStringLibrary.Conv_BoolToString` _array_element_4)))))))

(fn `SpawnPlayers`
  (bind _outactors (`GameplayStatics.GetAllActorsOfClass` "/Script/Engine.PlayerStart"))
  (for (_ _array_index) _outactors
    (`GameplayStatics.CreatePlayer` _array_index))
  (for (_array_element _array_index_2) _outactors
    (bind _returnvalue (`|SpawnActorFromClass` "/Game/ThirdPersonBP/Blueprints/ThirdPersonCharacter.ThirdPersonCharacter_C" (`self.GetTransform` _array_element) "Undefined" "OverrideRootScale" null null))
    (`Controller.Possess` (`GameplayStatics.GetPlayerController` _array_index_2) _returnvalue)
    (`PrimitiveComponent.SetMaterial` (`Character.Mesh` _returnvalue) 0 (`|GetArrayItem` (`self.PlayerMaterials`) _array_index_2))))

(fn `UserConstructionScript`)