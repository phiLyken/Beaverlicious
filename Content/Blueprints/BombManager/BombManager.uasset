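; BombManager tracks whether each bomb dropoff slot holds its matching pickup and decides the end-game effect.
; Every tick, VerifyBombSlots compares each DropoffPoint's current item class to the slot's expected class, switching its billboard between correct and false materials and rebuilding the sprite element at fixed size.
; EndGame re-verifies, then spawns a large explosion at BombPosition if all slots match, or a smaller TutorialParticleSystem effect otherwise.
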(event `self.ReceiveTick`
  (params (DeltaSeconds :type "Float (single-precision)"))
  (`self.VerifyBombSlots`))

(fn `EndGame`
  (bind _returnvalue (`self.K2_GetActorLocation` (`self.BombPosition`)))
  (`self.VerifyBombSlots`)
  (if (`self.AnySlotFalseOrEmpty`)
    (`GameplayStatics.SpawnEmitterAtLocation` "/Engine/Tutorial/SubEditors/TutorialAssets/TutorialParticleSystem.TutorialParticleSystem" _returnvalue (struct) (2.5 2.5 2.5))
    (else
      (`GameplayStatics.SpawnEmitterAtLocation` "/Game/FXVarietyPack/Particles/P_ky_explosion.P_ky_explosion" _returnvalue (struct) (5.0 5.0 5.0)))))

(fn `UserConstructionScript`)

(fn `VerifyBombSlots`
  (set `self.AnySlotFalseOrEmpty` false)
  (for _array_element (`self.BombSlots`)
    (bind (_dropoffpoint _matchingpickupclass) (break `/Game/Blueprints/BombManager/BombSlots` _array_element))
    (if (== (`GameplayStatics.GetObjectClass` (`/Game/PickupSystem/DropoffPoint_Base.CurrentItem` _dropoffpoint)) _matchingpickupclass)
      (bind _dropoffstatematerial (`/Game/PickupSystem/DropoffPoint_Base.DropoffStateMaterial` _dropoffpoint))
      (`PrimitiveComponent.SetMaterial` _dropoffstatematerial 0 "/Game/Blueprints/BombManager/CorrectBillboard.CorrectBillboard")
      (bind (_material _distancetoopacitycurve _bsizeisinscreenspace _basesizex _basesizey _distancetosizecurve) (break `MaterialSpriteElement` (`|GetArrayItem` (`MaterialBillboardComponent.Elements` _dropoffstatematerial))))
      (bind _array (`|MakeArray` (make `MaterialSpriteElement` _material _distancetoopacitycurve _bsizeisinscreenspace 80.0 80.0 _distancetosizecurve)))
      (`MaterialBillboardComponent.SetElements` _dropoffstatematerial _array)
      (else
        (set `self.AnySlotFalseOrEmpty` true)
        (`PrimitiveComponent.SetMaterial` _dropoffstatematerial 0 "/Game/Blueprints/BombManager/FalseBillboard.FalseBillboard")
        (`MaterialBillboardComponent.SetElements` _dropoffstatematerial _array)))))