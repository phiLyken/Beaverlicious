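; Attack controller that lets its owner stun nearby ThirdPersonCharacters by disabling their input.
; Attack scans all characters of that class, skipping the owner, and uses a squared-distance check against a range cached at BeginPlay.
; Tick counts down the stun duration and then re-enables input.
; Only one stunned actor and timer are tracked, so when several are hit, only the last one gets input back.
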(event `self.ReceiveBeginPlay`
  (set `self.SqrAttackRange` (`KismetMathLibrary.Square` (`self.AttackRange`))))

(event `self.ReceiveTick`
  (params (DeltaSeconds :type "Float (single-precision)"))
  (if (`KismetSystemLibrary.IsValid` (`self.StunnedActor`))
    (bind _output_get (set `self.StunTimer` (- (`self.StunTimer`) DeltaSeconds)))
    (`/Engine/EditorBlueprintResources/StandardMacros.CompareFloat` _output_get
      (:`==`
        _)
      (:`<`
        _))
    (`Actor.EnableInput` (`self.StunnedActor`) null)
    (set `self.StunnedActor` null)))

(fn `Attack`
  (bind _returnvalue (`self.GetOwner`))
  (bind _outactors (`GameplayStatics.GetAllActorsOfClass` "/Game/ThirdPersonBP/Blueprints/ThirdPersonCharacter.ThirdPersonCharacter_C"))
  (for _array_element _outactors
    (if (== _array_element _returnvalue)
      _
      (elif (>= (`self.SqrAttackRange`) (`KismetMathLibrary.Vector_DistanceSquared` (`Actor.K2_GetActorLocation` _array_element) (`Actor.K2_GetActorLocation` _returnvalue)))
        (bind _output_get (set `self.StunnedActor` _array_element))
        (`Actor.DisableInput` _output_get null)
        (set `self.StunTimer` (`self.StunDuration`))))))